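; Actor that cycles its skeletal mesh through animatronic characters, apparently for display in the HUD.
; On BeginPlay it starts UpdateMesh, which swaps the mesh to Chica, Gator and Freddy with a fixed delay before each change.
; UpdateMesh calls itself at the end to loop endlessly, reinitializing the pose on every swap.
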(event `self.ReceiveBeginPlay`
  (`self.UpdateMesh`))

(event `UpdateMesh`
  (`KismetSystemLibrary.Delay` 3.0)
  (`SkinnedMeshComponent.SetSkinnedAssetAndUpdate` (`self.SkeletalMesh`) "/Game/Animatronics_robots/Animations/Chica/Chica.Chica" true)
  (`KismetSystemLibrary.Delay` 3.0)
  (`SkinnedMeshComponent.SetSkinnedAssetAndUpdate` (`self.SkeletalMesh`) "/Game/Animatronics_robots/Animations/Gator/Gator.Gator" true)
  (`KismetSystemLibrary.Delay` 3.0)
  (`SkinnedMeshComponent.SetSkinnedAssetAndUpdate` (`self.SkeletalMesh`) "/Game/Animatronics_robots/Animations/Freddy/Freddy.Freddy" true)
  (`self.UpdateMesh`))

(fn `UserConstructionScript`)