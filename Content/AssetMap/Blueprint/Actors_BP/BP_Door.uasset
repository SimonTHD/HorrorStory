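; BP_Door is an interactive door that swings open or closed on a left mouse click while input is enabled.
; BoxColl overlaps enable and disable player-controller input on the actor and toggle the Icon's visibility, which each click also toggles.
; A timeline drives the Door's relative yaw.
; Its current track value, rather than the IsOpen flag it sets, decides whether to play or reverse.
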(event `self.BoxColl.OnComponentBeginOverlap`
  (params (OverlappedComponent :type "PrimitiveComponent Object Reference") (OtherActor :type "Actor Object Reference") (OtherComp :type "PrimitiveComponent Object Reference") (OtherBodyIndex :type Integer) (bFromSweep :type Boolean) (SweepResult :type "HitResult Structure (by ref)"))
  (`self.EnableInput` (`GameplayStatics.GetPlayerController` 0))
  (`SceneComponent.ToggleVisibility` (`self.icon`) false :!label _label))

(event `self.BoxColl.OnComponentEndOverlap`
  (params (OverlappedComponent :type "PrimitiveComponent Object Reference") (OtherActor :type "Actor Object Reference") (OtherComp :type "PrimitiveComponent Object Reference") (OtherBodyIndex :type Integer))
  (`self.DisableInput` (`GameplayStatics.GetPlayerController` 0))
  (goto _label))

(event `Key|LeftMouseButton`
  (params (Key :type "Key Structure"))
  (:`Pressed`
    (`SceneComponent.ToggleVisibility` (`self.icon`) false)))

(event `Key|LeftMouseButton`
  (params (Key :type "Key Structure"))
  (:`Pressed`
    (if (< -1.0 (stale _newtrack_0))
      (set `self.IsOpen?` true)
      (bind (_direction _newtrack_0) (`Timeline|Timeline_0` :!label _label_2)
        (:`Update`
          (`SceneComponent.K2_SetRelativeRotation` (`self.Door`) (`KismetMathLibrary.MakeRotator` 0.0 0.0 _newtrack_0) false false)))
      (else
        (set `self.IsOpen?` false)
        (goto _label_2 :!via `Reverse`)))))

(fn `UserConstructionScript`)