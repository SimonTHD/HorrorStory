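; Game mode for the flashlight horror character that implements an hour-style clock with a finish time, apparently an unfinished prototype.
; BeginPlay caches the game instance and player character, then calls UpdateClock once after a delay.
; UpdateClock advances the hour with twelve-hour wraparound and prints either the time or a finish message, without rescheduling itself.
; A disconnected duplicate of the clock logic remains unused.
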(event `self.ReceiveBeginPlay`
  (bind _asgi_game (cast `/Game/Animatronics_robots/Sprint_6/GI_Game` (`GameplayStatics.GetGameInstance`)))
  (set `self.GiRef` _asgi_game)
  (bind _asbp_flashlight_horror_character (cast `/Game/HorrorCharacter/HorrorCharacter/Blueprints/BP_FlashlightHorrorCharacter` (`GameplayStatics.GetPlayerCharacter` 0)))
  (set `self.CharRef` _asbp_flashlight_horror_character)
  (`KismetSystemLibrary.Delay` 30.0)
  (`self.UpdateClock`))

(event `UpdateClock`
  (set `self.currentTime` (+ (`self.currentTime`) 1))
  (if (> (`self.currentTime`) 12)
    (set `self.currentTime` 1))
  (if (== (`self.currentTime`) (`self.finishTime`))
    (`KismetSystemLibrary.PrintString` "Finish")
    (else
      (`KismetSystemLibrary.PrintString` (`KismetStringLibrary.Conv_IntToString` (`self.currentTime`))))))

(fn `UserConstructionScript`)