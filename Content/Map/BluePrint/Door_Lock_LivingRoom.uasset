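; Locked living room door that the player opens and closes by interacting with it.
; While locked, interaction checks the BP_FlashlightHorrorCharacter for the living room key, then either unlocks permanently and toggles the door or updates the character's journal.
; A DoorOpen timeline drives the carved door mesh's yaw, playing forward to open and reversing to close.
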(event `/Game/ImmersiveFlashlight/Interface/InteractInterface.Interact`
  (if (`self.isKeyOpen?`)
    ;[1 1 1] System of the door
    (if (`self.isOpen?`) :!label _label
      (`self.CloseDoor`)
      (set `self.isOpen?` false)
      (else
        (`self.OpenDoor`)
        (set `self.isOpen?` true)))
    (else
      (bind _asbp_flashlight_horror_character (cast `/Game/HorrorCharacter/HorrorCharacter/Blueprints/BP_FlashlightHorrorCharacter` (`GameplayStatics.GetPlayerPawn` 0)))
      (if (`/Game/HorrorCharacter/HorrorCharacter/Blueprints/BP_FlashlightHorrorCharacter.keyLivingRoom?` _asbp_flashlight_horror_character)
        (set `self.isKeyOpen?` true)
        (goto _label)
        (else
          ;[1 1 1] Not Key
          (`/Game/HorrorCharacter/HorrorCharacter/Blueprints/BP_FlashlightHorrorCharacter.UpdateJournal` _asbp_flashlight_horror_character "NewEnumerator6"))))))

(event `OpenDoor`
  ;[1 1 1] Door Open
  (bind (_direction _newtrack_0) (`Timeline|DoorOpen` :!label _label_2)
    (:`Update`
      (`SceneComponent.K2_SetRelativeRotation` (`self.SM_DoorCarved`) (`KismetMathLibrary.MakeRotator` 0.0 0.0 _newtrack_0) false false))))

(event `CloseDoor`
  ;[1 1 1] Door Open
  (goto _label_2 :!via `Reverse`))

(fn `UserConstructionScript`)