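; Animatronic enemy for a night-based horror game that wakes on a schedule and triggers a jumpscare on contact with the player.
; Construction pulls mesh, scale and AI controller from a data table row.
; From its start night onward, a looping timer rolls a weighted chance against the gamemode clock, then fires the AI activation dispatcher once.
; Getters expose door and target points; the jumpscare query always returns false, and PlayJumpscare only pauses the game.
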(event `self.ReceiveBeginPlay`
  (bind _asbp_flashlight_horror_character_gamemode (cast `/Game/HorrorCharacter/HorrorCharacter/Blueprints/BP_FlashlightHorrorCharacterGamemode` (`GameplayStatics.GetGameMode`)))
  (set `self.GMRef` _asbp_flashlight_horror_character_gamemode)
  (bind _asgi_game (cast `/Game/Animatronics_robots/Sprint_6/GI_Game` (`GameplayStatics.GetGameInstance`)))
  (if (>= (`/Game/Animatronics_robots/Sprint_6/GI_Game.CurrentNight` _asgi_game) (`self.StartNight`))
    (set `self.StartTime` (`KismetMathLibrary.RandomIntegerInRange` 1 1))
    (`KismetSystemLibrary.K2_SetTimer` null "CheckCanBeActive" 4.0 true)))

(event `/Game/Animatronics_robots/Sprint_6/Interface/BI_Animatronics.PlayJumpscare`
  (`GameplayStatics.SetGamePaused` true))

(event `/Game/Animatronics_robots/Sprint_6/Interface/BI_Animatronics.SetAnimatronicsJumpscare`
  (params (JumpscareActive :type Boolean))
  (set `self.CanJumpScare?` JumpscareActive))

(event `self.Box.OnComponentBeginOverlap`
  (params (OverlappedComponent :type "PrimitiveComponent Object Reference") (OtherActor :type "Actor Object Reference") (OtherComp :type "PrimitiveComponent Object Reference") (OtherBodyIndex :type Integer) (bFromSweep :type Boolean) (SweepResult :type "HitResult Structure (by ref)"))
  (cast `/Game/HorrorCharacter/HorrorCharacter/Blueprints/BP_FlashlightHorrorCharacter` OtherActor)
  (`/Engine/EditorBlueprintResources/StandardMacros.DoOnce` false
    (:`Completed`
      (`self.OnJumpScare`))))

(fn `AnimatronicsRef`
  (returns (Ref :type "/Game/Animatronics_robots/Sprint_6/AI/BP_Animatronics Object Reference"))
  (return self))

(fn `CanAnimatronicsJumpscare?`
  (returns (`JumpScareActive?` :type Boolean))
  (return false))

(fn `CheckCanBeActive`
  (bind _currenttime (`/Game/HorrorCharacter/HorrorCharacter/Blueprints/BP_FlashlightHorrorCharacterGamemode.currentTime` (`self.GMRef`)))
  (if (and (`KismetMathLibrary.RandomBoolWithWeight` 0.5) (>= (select `bool` (== _currenttime 12) :`false` _currenttime :`true` (- _currenttime 12)) (`self.StartTime`)))
    (`KismetSystemLibrary.K2_ClearTimer` null "CheckCanBeActive")
    (`self.ActivateAISequence`)))

(fn `GetAnimatronicsDoorIndex`
  (returns (DoorIndex :type Integer))
  (return (`self.DoorIndex`)))

(fn `GetAnimatronicsDoorRef`
  (returns (Door :type "/Game/AssetMap/Blueprint/Actors_BP/BP_Door Object Reference"))
  (return (`self.DoorRef`)))

(fn `GetAnimatronicsTargetPoint`
  (returns (TargetPoints :type "Array of /Game/Animatronics_robots/Sprint_6/AI/BP_TargetPoints Object Reference"))
  (return (`self.TargetPoints`)))

(fn `SetupModel`
  (bind (_animatronicsdata_datatable _animatronicsdata_rowname) (break `DataTableRowHandle` (`self.AnimatronicsData`)))
  (bind _returnvalue (`|GetDataTableRow` _animatronicsdata_datatable _animatronicsdata_rowname)
    (:`then`
      (bind (_name _basestarttime _basestartnight _model _worldscale _aicontroller) (break `/Game/Animatronics_robots/Sprint_6/Struct/S_Animatronics_data` _returnvalue))
      (`SkinnedMeshComponent.SetSkinnedAssetAndUpdate` (`self.Mesh`) _model true)
      (`self.SetActorScale3D` _worldscale)
      (set `self.AIControllerClass` _aicontroller))))

(fn `UserConstructionScript`
  (`self.SetupModel`))