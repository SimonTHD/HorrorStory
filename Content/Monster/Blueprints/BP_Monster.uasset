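; Monster AI for a horror game that wanders slowly and chases the flashlight character on sight.
; BeginPlay starts a loop of moves to random nearby reachable points, which pauses while IsChasing is set.
; PawnSensing starts the chase, and a retriggerable delay returns it to wandering shortly after sightings stop.
; Tick switches walk speed from IsChasing, and reaching the player fires the OnJumpScare dispatcher once.
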(event `self.ReceiveBeginPlay`
  (bind _ischasing_ (`self.isChasing?`))
  (`|AIMoveTo` self (`NavigationSystemV1.K2_GetRandomReachablePointInRadius` (`self.K2_GetActorLocation`) 1000.0 null null) null :!label _label
    (:`OnSuccess`
      _)
    (:`OnFail`
      _))
  (if (not _ischasing_) :!label _label_2
    (`KismetSystemLibrary.Delay` 5.0)
    (if _ischasing_
      _
      (else
        (goto _label))))
  (`KismetSystemLibrary.Delay` 2.0)
  (goto _label_2))

(event `self.PawnSensing.OnSeePawn`
  (params (Pawn :type "Pawn Object Reference"))
  (bind _asbp_flashlight_horror_character (cast `/Game/HorrorCharacter/HorrorCharacter/Blueprints/BP_FlashlightHorrorCharacter` Pawn))
  (`|AIMoveTo` self (0.0 0.0 0.0) _asbp_flashlight_horror_character
    (:`then`
      (set `self.isChasing?` true)
      (`KismetSystemLibrary.RetriggerableDelay` 3.0)
      (set `self.isChasing?` false)
      (goto _label))
    (:`OnSuccess`
      (`/Engine/EditorBlueprintResources/StandardMacros.DoOnce` false
        (:`Completed`
          (`self.OnJumpScare`))))
    (:`OnFail`
      (set `self.isChasing?` false))))

(event `self.ReceiveTick`
  (params (DeltaSeconds :type "Float (single-precision)"))
  (bind _charactermovement (`self.CharacterMovement`))
  (if (`self.isChasing?`)
    (set `CharacterMovementComponent.MaxWalkSpeed` 400.0 _charactermovement)
    (else
      (set `CharacterMovementComponent.MaxWalkSpeed` 40.0 _charactermovement))))

(fn `UserConstructionScript`)